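; BP_Death is a hazard actor with a moving component and a death zone that sends the player character back to a marker.
; When BP_BodyChar overlaps Trigger, a Timeline plays and lerps the Er component from the Start location to the Target location, printing a debug string.
; When BP_BodyChar overlaps Death, it is moved to the Billboard location without sweep, acting as a simple respawn.
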(event OnComponentBeginOverlap(Trigger)
  (params (OverlappedComponent :type Primitive%20Component%20Object%20Reference) (OtherActor :type Actor%20Object%20Reference) (OtherComp :type Primitive%20Component%20Object%20Reference) (OtherBodyIndex :type Integer) (bFromSweep :type Boolean) (SweepResult :type Hit%20Result%20Structure%20%28by%20ref%29))
  (Utilities|Casting|CastToBP_BodyChar OtherActor)
  (Development|PrintString "casting")
  (bind _z (Timeline|Timeline Play)
    (:Update
      (Transformation|SetWorldLocation (Variables|Default|Geter) (Math|Vector|Lerp(Vector) (Transformation|GetWorldLocation (Variables|Default|GetStart)) (Transformation|GetWorldLocation (Variables|Default|GetTarget)) _z) false false))))

(event OnComponentBeginOverlap(Death)
  (params (OverlappedComponent :type Primitive%20Component%20Object%20Reference) (OtherActor :type Actor%20Object%20Reference) (OtherComp :type Primitive%20Component%20Object%20Reference) (OtherBodyIndex :type Integer) (bFromSweep :type Boolean) (SweepResult :type Hit%20Result%20Structure%20%28by%20ref%29))
  (bind _asbp_body_char (Utilities|Casting|CastToBP_BodyChar OtherActor))
  (Transformation|SetActorLocation _asbp_body_char (Transformation|GetWorldLocation (Variables|Default|GetBillboard)) false false))

(event EventBeginPlay)

(event EventTick
  (params (DeltaSeconds :type Float%20%28single-precision%29)))

(fn ConstructionScript)